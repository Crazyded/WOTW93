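; BP_Weapon_Revolver is a revolver weapon Blueprint that fires a hitscan shot using the player's revolver ammo.
; Its Fire event reads AmmoRevolver on BP_Player, spends a round, line-traces forward from an Arrow component and damages the hit actor.
; A gunshot sound plays at the weapon, while an empty-clip sound plays at the world origin when ammo is depleted.
; Debug trace drawing and a debug print are left in.
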(event `self.Fire`
  (bind _arrow (`self.Arrow`))
  (bind _returnvalue (`SceneComponent.K2_GetComponentLocation` _arrow))
  (bind _asbp_player (cast `/Game/Blueprints/DEBUG_PLAYER/BP_Player` (`GameplayStatics.GetPlayerCharacter` 0)))
  (if (> (`/Game/Blueprints/DEBUG_PLAYER/BP_Player.AmmoRevolver` _asbp_player) 0)
    (`/Engine/EditorBlueprintResources/StandardMacros.DecrementInt` (`/Game/Blueprints/DEBUG_PLAYER/BP_Player.AmmoRevolver` _asbp_player)
      (:`  `
        (`KismetSystemLibrary.PrintString` "AttackRevolver")
        (bind _outhit (`KismetSystemLibrary.LineTraceSingle` :`Start` _returnvalue :`End` (+ _returnvalue (* (`SceneComponent.GetForwardVector` _arrow) 1000.0)) :`TraceChannel` "TraceTypeQuery1" :`DrawDebugType` "ForDuration"))
        (`GameplayStatics.PlaySoundAtLocation` "/Game/Audio/Weapons/Revolver/magnum_shoot.magnum_shoot" (`self.K2_GetActorLocation`) (struct) 1.0 1.0 0.0 null null null null)
        (`GameplayStatics.ApplyDamage` (`.HitActor` (`GameplayStatics.BreakHitResult` _outhit)) 50.0)))
    (else
      (`GameplayStatics.PlaySoundAtLocation` "/Game/Audio/Weapons/clipempty_pistol.clipempty_pistol" (0.0 0.0 0.0) (struct) 1.0 1.0 0.0 null null null null))))

(fn `UserConstructionScript`
  (`parent.UserConstructionScript`))