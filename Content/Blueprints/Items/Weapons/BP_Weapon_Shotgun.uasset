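; Shotgun weapon Blueprint whose Fire event simulates a multi-pellet blast with a loop of line traces.
; Each trace runs forward from the Arrow component on the Visibility channel, with spread from random world-axis offsets on its end point.
; The fire sound plays at the actor's location on every loop iteration.
; Traces draw debug lines and their hit results are unused, so no damage is applied.
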(event `self.Fire`
  (bind _returnvalue (`KismetMathLibrary.RandomFloatInRange` -10.0 10.0))
  (bind _arrow (`self.Arrow`))
  (bind _returnvalue_2 (`SceneComponent.K2_GetComponentLocation` _arrow))
  (`KismetSystemLibrary.PrintString` "AttackShotgun")
  (for _ (range 10)
    (`KismetSystemLibrary.LineTraceSingle` :`Start` _returnvalue_2 :`End` (`KismetMathLibrary.MakeVector` (+ (.x (+ _returnvalue_2 (* (`SceneComponent.GetForwardVector` _arrow) 1000.0))) _returnvalue) (+ _returnvalue (.y (+ _returnvalue_2 (* (`SceneComponent.GetForwardVector` _arrow) 1000.0)))) (+ (.z (+ _returnvalue_2 (* (`SceneComponent.GetForwardVector` _arrow) 1000.0))) _returnvalue)) :`TraceChannel` "TraceTypeQuery1" :`DrawDebugType` "ForDuration")
    (`GameplayStatics.PlaySoundAtLocation` "/Game/Audio/Weapons/Shotgun/shotgun_fire_1.shotgun_fire_1" (`self.K2_GetActorLocation`) (struct) 1.0 1.0 0.0 null null null null)))

(fn `UserConstructionScript`
  (`parent.UserConstructionScript`))